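; BP_Antagonist is an antagonist actor whose state follows a danger meter.
; Each Tick picks one of three states from the meter, switching at three-quarters and at full, and shows the mesh in all but the lowest.
; Functions reset the meter and state or nudge the meter up or down by five percent, without clamping.
; The PawnSensing sight event only casts to FirstPersonCharacter and takes no further action.
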(event `self.ReceiveTick`
  (params (DeltaSeconds :type "Float (single-precision)"))
  (bind _antagonist_state (`self.Antagonist_State`))
  (bind _staticmeshcomponent (`self.StaticMeshComponent`))
  (`|ExecutionSequence`
    (:`then_0`
      (if (>= (`self.DangerMeter_Percent`) 0.75)
        (if (>= (`self.DangerMeter_Percent`) 1.0)
          (if (not (`|EnumEquality` _antagonist_state "NewEnumerator2"))
            (set `self.Antagonist_State` "NewEnumerator2"))
          (elif (not (`|EnumEquality` _antagonist_state "NewEnumerator1"))
            (set `self.Antagonist_State` "NewEnumerator1")))
        (elif (not (`|EnumEquality` (`self.Antagonist_State`) "NewEnumerator0"))
          (set `self.Antagonist_State` "NewEnumerator0"))))
    (:`then_1`
      (if (`|EnumEquality` (`self.Antagonist_State`) "NewEnumerator0")
        (`SceneComponent.SetVisibility` _staticmeshcomponent false false)
        (else
          (`SceneComponent.SetVisibility` _staticmeshcomponent true false))))))

(event `self.PawnSensing.OnSeePawn`
  (params (Pawn :type "Pawn Object Reference"))
  (cast `/Game/Jett/FirstPersonBP/Blueprints/FirstPersonCharacter` Pawn))

(fn `Decrease Danger Meter 5%`
  (set `self.DangerMeter_Percent` (- (`self.DangerMeter_Percent`) 0.05)))

(fn `Increase Danger Meter 5%`
  (set `self.DangerMeter_Percent` (+ (`self.DangerMeter_Percent`) 0.05)))

(fn `Init`
  (set `self.Antagonist_State` "NewEnumerator0")
  (set `self.DangerMeter_Percent` 0.0))

(fn `UserConstructionScript`)