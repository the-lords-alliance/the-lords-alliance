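; BP_ExitHint is an exit hint actor whose eight point lights show which keys the player has collected.
; GenOn finds the Player with GetActorOfClass and lights the point light matching each held key flag, from HasKey through the color-named keys.
; It reads the flags only when GenOn fires, and GenOff switches all eight lights off.
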(event `GenOn`
  (bind _returnvalue (`GameplayStatics.GetActorOfClass` "/Game/Jett/FirstPersonBP/Player.Player_C"))
  (if (`/Game/Jett/FirstPersonBP/Player.HasKey` _returnvalue)
    (`LightComponent.SetIntensity` (`self.PointLight`) 1000.0))
  (if (`/Game/Jett/FirstPersonBP/Player.HasOrangeKey` _returnvalue)
    (`LightComponent.SetIntensity` (`self.PointLight1`) 1000.0))
  (if (`/Game/Jett/FirstPersonBP/Player.HasYellowKey` _returnvalue)
    (`LightComponent.SetIntensity` (`self.PointLight2`) 1000.0))
  (if (`/Game/Jett/FirstPersonBP/Player.HasLimeKey` _returnvalue)
    (`LightComponent.SetIntensity` (`self.PointLight3`) 1000.0))
  (if (`/Game/Jett/FirstPersonBP/Player.HasGreenKey` _returnvalue)
    (`LightComponent.SetIntensity` (`self.PointLight4`) 1000.0))
  (if (`/Game/Jett/FirstPersonBP/Player.HasLightBlueKey` _returnvalue)
    (`LightComponent.SetIntensity` (`self.PointLight5`) 1000.0))
  (if (`/Game/Jett/FirstPersonBP/Player.HasBlueKey` _returnvalue)
    (`LightComponent.SetIntensity` (`self.PointLight6`) 1000.0))
  (if (`/Game/Jett/FirstPersonBP/Player.HasPurpleKey` _returnvalue)
    (`LightComponent.SetIntensity` (`self.PointLight7`) 1000.0)))

(event `GenOff`
  (`LightComponent.SetIntensity` (`self.PointLight`) 0.0)
  (`LightComponent.SetIntensity` (`self.PointLight1`) 0.0)
  (`LightComponent.SetIntensity` (`self.PointLight2`) 0.0)
  (`LightComponent.SetIntensity` (`self.PointLight3`) 0.0)
  (`LightComponent.SetIntensity` (`self.PointLight4`) 0.0)
  (`LightComponent.SetIntensity` (`self.PointLight5`) 0.0)
  (`LightComponent.SetIntensity` (`self.PointLight6`) 0.0)
  (`LightComponent.SetIntensity` (`self.PointLight7`) 0.0))

(fn `UserConstructionScript`)