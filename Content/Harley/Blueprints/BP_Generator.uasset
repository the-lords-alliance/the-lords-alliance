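; BP_Generator is an interactable generator that the player fuels and switches on to initialise the level's BP_Light actors.
; Box overlaps show state-based HUDTooltips prompts and gate the Interact input, with fuel granted through SetHasFuel.
; Switching on also raises the NewBP_Antagonist's danger meter, then tells it to attack the generator after a minute's delay.
; TurnOffGen clears the on state and notifies the lights, but this graph never runs it.
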(event `self.ReceiveBeginPlay`
  (bind _returnvalue (`|CreateWidget` "/Game/Harley/Blueprints/HUDTooltips.HUDTooltips_C" (`GameplayStatics.GetPlayerController` 0)))
  (`UserWidget.AddToViewport` _returnvalue 0))

(event `self.Box.OnComponentEndOverlap`
  (params (OverlappedComponent :type "PrimitiveComponent Object Reference") (OtherActor :type "Actor Object Reference") (OtherComp :type "PrimitiveComponent Object Reference") (OtherBodyIndex :type Integer))
  (set `self.IsOverlapped` false)
  (set `self.MessageVis` "Hidden")
  (`self.EnableInput` (`GameplayStatics.GetPlayerController` 0))
  (bind _foundwidgets (`WidgetBlueprintLibrary.GetAllWidgetsOfClass` "/Game/Harley/Blueprints/HUDTooltips.HUDTooltips_C"))
  (`/Game/Harley/Blueprints/HUDTooltips.OnMessage` _foundwidgets (`self.MessageVis`) ""))

(event `self.Box.OnComponentBeginOverlap`
  (params (OverlappedComponent :type "PrimitiveComponent Object Reference") (OtherActor :type "Actor Object Reference") (OtherComp :type "PrimitiveComponent Object Reference") (OtherBodyIndex :type Integer) (bFromSweep :type Boolean) (SweepResult :type "HitResult Structure (by ref)"))
  (set `self.IsOverlapped` true)
  (set `self.MessageVis` "Visible")
  (`self.EnableInput` (`GameplayStatics.GetPlayerController` 0))
  (bind _foundwidgets (`WidgetBlueprintLibrary.GetAllWidgetsOfClass` "/Game/Harley/Blueprints/HUDTooltips.HUDTooltips_C" false))
  (if (`self.Fueled`)
    (`/Game/Harley/Blueprints/HUDTooltips.OnMessage` _foundwidgets (`self.MessageVis`) "Push E to turn on \nthe generator")
    (elif (`self.HasFuel`)
      (`/Game/Harley/Blueprints/HUDTooltips.OnMessage` _foundwidgets (`self.MessageVis`) "Push E to turn put the fuel \nin the generator")
      (else
        (`/Game/Harley/Blueprints/HUDTooltips.OnMessage` _foundwidgets (`self.MessageVis`) "You will need to find \nfuel for this first")))))

(event `InputAction|Interact`
  (params (Key :type "Key Structure"))
  (:`Pressed`
    (if (`self.IsOverlapped`)
      (if (`self.Fueled`)
        (set `self.IsOn` true)
        (bind _output_get (set `self.MessageVis` "Hidden"))
        (`/Game/Harley/Blueprints/HUDTooltips.OnMessage` (stale `self.Box.OnComponentBeginOverlap` _foundwidgets) _output_get "")
        (bind _outactors (`GameplayStatics.GetAllActorsOfClass` "/Game/Harley/Blueprints/BP_Light.BP_Light_C"))
        (`/Game/Harley/Blueprints/BP_Light.GeneratorInit` _outactors)
        (`/Game/Jacob/BP_InitJacob.Init` (`self.Target`))
        (bind _returnvalue (`GameplayStatics.GetActorOfClass` "/Game/Jacob/NewBP_Antagonist.NewBP_Antagonist_C"))
        (`/Game/Jacob/NewBP_Antagonist.Increase Danger Meter 5%` _returnvalue)
        (`KismetSystemLibrary.Delay` 60.0)
        (bind _returnvalue_2 (`GameplayStatics.GetActorOfClass` "/Game/Jacob/NewBP_Antagonist.NewBP_Antagonist_C"))
        (`/Game/Jacob/NewBP_Antagonist.Attack_Generator` _returnvalue_2)
        (elif (`self.HasFuel`)
          (set `self.Fueled` true)
          (`/Game/Harley/Blueprints/HUDTooltips.OnMessage` (stale `self.Box.OnComponentBeginOverlap` _foundwidgets) (`self.MessageVis`) "Push E to turn on \nthe generator"))))))

(fn `SetHasFuel`
  (set `self.HasFuel` true))

(fn `TurnOffGen`
  (set `self.IsOn` false)
  (bind _outactors (`GameplayStatics.GetAllActorsOfClass` "/Game/Harley/Blueprints/BP_Light.BP_Light_C"))
  (`/Game/Harley/Blueprints/BP_Light.GeneratorOff` _outactors))

(fn `UserConstructionScript`)