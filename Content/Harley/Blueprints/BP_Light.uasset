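; An interactable light actor that the player toggles with the Interact input while overlapping it, with a HUD tooltip shown during overlap.
; SetIntensity records a start, target and period, and Tick applies a cubic-eased, frame-rate-independent lerp to the point light, though every current caller passes zero for an instant change.
; GeneratorInit turns it on when OnStart is set, and its sphere raises NewBP_Antagonist's danger meter on overlap.
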(event `self.ReceiveActorBeginOverlap`
  (params (OtherActor :type "Actor Object Reference"))
  (set `self.isOverlapped` true)
  (`self.EnableInput` (`GameplayStatics.GetPlayerController` 0))
  (bind _foundwidgets (`WidgetBlueprintLibrary.GetAllWidgetsOfClass` "/Game/Harley/Blueprints/HUDTooltips.HUDTooltips_C"))
  (`/Game/Harley/Blueprints/HUDTooltips.OnMessage` _foundwidgets "Visible" "Push E to turn on"))

(event `self.ReceiveActorEndOverlap`
  (params (OtherActor :type "Actor Object Reference"))
  (set `self.isOverlapped` false)
  (`self.DisableInput` (`GameplayStatics.GetPlayerController` 0))
  (bind _foundwidgets (`WidgetBlueprintLibrary.GetAllWidgetsOfClass` "/Game/Harley/Blueprints/HUDTooltips.HUDTooltips_C"))
  (`/Game/Harley/Blueprints/HUDTooltips.OnMessage` _foundwidgets "Hidden" ""))

(event `self.ReceiveTick`
  (params (DeltaSeconds :type "Float (single-precision)"))
  (bind _pointlight (`self.PointLight`))
  ;[1 1 1] Finds the Lerp without being affected by FPS
  (if (`self.Changing`)
    (bind _output_get (set `self.Lerp Factor` (+ (`self.Lerp Factor`) (/ DeltaSeconds (`self.Time Period`)))))
    ;[1 1 1] Gets the intensity values to the New Intensity pins in the Set Intensity nodes. (
    (if (>= _output_get 1.0)
      (`LightComponent.SetIntensity` _pointlight (`self.Target Intensity`))
      (set `self.Changing` true)
      (else
        (`LightComponent.SetIntensity` _pointlight (`KismetMathLibrary.Lerp` (`self.Start Intensity`) (`self.Target Intensity`) (`KismetMathLibrary.MultiplyMultiply_FloatFloat` (`self.Lerp Factor`) 3.0)))))))

(event `InputAction|Interact` :consume false
  (params (Key :type "Key Structure"))
  (:`Pressed`
    (if (`self.IsOverlapped`)
      (if (<= (`LightComponentBase.Intensity` (`self.PointLight`)) 0.0)
        (`self.Set Intensity` 10000.0)
        (else
          (`self.Set Intensity` 0.0))))))

(event `GeneratorInit`
  (if (`self.OnStart`)
    (`self.Set Intensity` 10000.0)))

(event `self.ReceiveBeginPlay`
  (`self.Set Intensity` (`self.Intensity`)))

(event `self.Sphere.OnComponentBeginOverlap`
  (params (OverlappedComponent :type "PrimitiveComponent Object Reference") (OtherActor :type "Actor Object Reference") (OtherComp :type "PrimitiveComponent Object Reference") (OtherBodyIndex :type Integer) (bFromSweep :type Boolean) (SweepResult :type "HitResult Structure (by ref)"))
  (bind _asnew_bp_antagonist (cast `/Game/Jacob/NewBP_Antagonist` OtherActor))
  (`/Game/Jacob/NewBP_Antagonist.Increase Danger Meter 5%` _asnew_bp_antagonist))

(fn `Set Intensity`
  (params (Intensity :type "Float (double-precision)") (`Time Period` :type "Float (double-precision)"))
  (set `self.Target Intensity` Intensity)
  (set `self.Time Period` `Time Period`)
  (set `self.Start Intensity` (`LightComponentBase.Intensity` (`self.PointLight`)))
  (set `self.Changing` true)
  (if (< (`self.Time Period`) 0.0001)
    (set `self.Lerp Factor` 1.0)
    (else
      (set `self.Lerp Factor` 0.0))))

(fn `UserConstructionScript`)