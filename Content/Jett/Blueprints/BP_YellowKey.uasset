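; BP_YellowKey is a yellow key pickup that the player collects with the Interact input.
; Overlap begin and end toggle the actor's input and show or hide a "Push E to pick Up" prompt through HUDTooltips, created on BeginPlay.
; Interact destroys the key and sets HasYellowKey on the overlapping Player.
; A second, Gate-based Interact path remains, but its open and close logic never runs.
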(event `self.ReceiveBeginPlay`
  (bind _returnvalue (`|CreateWidget` "/Game/Harley/Blueprints/HUDTooltips.HUDTooltips_C" (`GameplayStatics.GetPlayerController` 0)))
  (`UserWidget.AddToViewport` _returnvalue 0))

(event `InputAction|Interact`
  (params (Key :type "Key Structure"))
  (:`Pressed`
    (`/Engine/EditorBlueprintResources/StandardMacros.Gate` true
      (:`Exit`
        (`self.K2_DestroyActor`)))))

(event `CustomEvent_2`
  (bind _returnvalue (`|CreateWidget` "/Game/Harley/Blueprints/HUDTooltips.HUDTooltips_C" (`GameplayStatics.GetPlayerController` 0)))
  (`UserWidget.AddToViewport` _returnvalue 0))

(event `self.ReceiveActorEndOverlap`
  (params (OtherActor :type "Actor Object Reference"))
  (`self.DisableInput` (`GameplayStatics.GetPlayerController` 0))
  (bind _foundwidgets (`WidgetBlueprintLibrary.GetAllWidgetsOfClass` "/Game/Harley/Blueprints/HUDTooltips.HUDTooltips_C"))
  (`/Game/Harley/Blueprints/HUDTooltips.OnMessage` _foundwidgets "Hidden" "Push E to pick Up"))

(event `self.ReceiveActorBeginOverlap`
  (params (OtherActor :type "Actor Object Reference"))
  (`self.EnableInput` (`GameplayStatics.GetPlayerController` 0))
  (bind _foundwidgets (`WidgetBlueprintLibrary.GetAllWidgetsOfClass` "/Game/Harley/Blueprints/HUDTooltips.HUDTooltips_C"))
  (`/Game/Harley/Blueprints/HUDTooltips.OnMessage` _foundwidgets "Visible" "Push E to pick Up"))

(event `InputAction|Interact`
  (params (Key :type "Key Structure"))
  (:`Pressed`
    (`self.K2_DestroyActor`)
    (bind _asplayer (cast `/Game/Jett/FirstPersonBP/Player` (stale `self.ReceiveActorBeginOverlap` OtherActor)))
    (set `/Game/Jett/FirstPersonBP/Player.HasYellowKey` true _asplayer)))

(fn `UserConstructionScript`)