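; BP_HidingSpot is an interactable spot that moves the player into its position to hide.
; Begin and end overlap enable or disable its input for player controller 0 and show or hide a "Push E to hide" prompt through HUDTooltips widgets.
; Pressing Interact casts the actor from begin overlap to Player and sets its location to the spot root's X and Y at a fixed height.
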(event `self.ReceiveActorEndOverlap`
  (params (OtherActor :type "Actor Object Reference"))
  (`self.DisableInput` (`GameplayStatics.GetPlayerController` 0))
  (bind _foundwidgets (`WidgetBlueprintLibrary.GetAllWidgetsOfClass` "/Game/Harley/Blueprints/HUDTooltips.HUDTooltips_C"))
  (`/Game/Harley/Blueprints/HUDTooltips.OnMessage` _foundwidgets "Hidden" "Push E to hide"))

(event `self.ReceiveActorBeginOverlap`
  (params (OtherActor :type "Actor Object Reference"))
  (`self.EnableInput` (`GameplayStatics.GetPlayerController` 0))
  (bind _foundwidgets (`WidgetBlueprintLibrary.GetAllWidgetsOfClass` "/Game/Harley/Blueprints/HUDTooltips.HUDTooltips_C"))
  (`/Game/Harley/Blueprints/HUDTooltips.OnMessage` _foundwidgets "Visible" "Push E to hide"))

(event `InputAction|Interact`
  (params (Key :type "Key Structure"))
  (bind (_returnvalue_x _returnvalue_y) (`KismetMathLibrary.BreakVector` (`SceneComponent.K2_GetComponentLocation` (`self.DefaultSceneRoot`))))
  (:`Pressed`
    (bind _asplayer (cast `/Game/Jett/FirstPersonBP/Player` (stale `self.ReceiveActorBeginOverlap` OtherActor)))
    (`self.K2_SetActorRelativeLocation` _asplayer (`KismetMathLibrary.MakeVector` _returnvalue_x _returnvalue_y 200.0) false false)))

(fn `UserConstructionScript`)